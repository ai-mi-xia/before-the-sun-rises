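; Gem pickup actor that boosts the jump velocity of any third-person character overlapping its pickup radius.
; The overlap calls a server add-gems event, plays a 2D sound, then destroys the gem and radius components while keeping the actor.
; The server events for adding gems and giving a key only cast the player controller so far.
; Gem counting, max-stamina and popup widget logic is left disconnected.
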(event OnComponentBeginOverlap(PickUpRadius)
  (params (OverlappedComponent :type Primitive%20Component%20Object%20Reference) (OtherActor :type Actor%20Object%20Reference) (OtherComp :type Primitive%20Component%20Object%20Reference) (OtherBodyIndex :type Integer) (bFromSweep :type Boolean) (SweepResult :type Hit%20Result%20Structure%20%28by%20ref%29))
  ;[1 1 1] Pickup Gem
  (Collision|IgnoreActorwhenMoving (Variables|Default|GetPickUpRadius) 0 false)
  (bind _asbp_third_person_character (Utilities|Casting|CastToBP_ThirdPerson_Character OtherActor))
  ;;[1 1 1] Change Jump Velocity of Character that picked it up
  (Variables|/Script/Engine.CharacterMovementComponent|SetJumpZVelocity (Variables|/Script/Engine.Character|GetCharacterMovement _asbp_third_person_character) (+ (Variables|/Script/Engine.CharacterMovementComponent|GetJumpZVelocity (Variables|/Script/Engine.Character|GetCharacterMovement _asbp_third_person_character)) 1e+02))
  (CallFunction|ServerAddGems OtherActor) ; issue here on spawn
  (Audio|PlaySound2D "/Engine/VREditor/Sounds/UI/Click_on_Button_Cue.Click_on_Button_Cue" 1.0 1.0 0.0 0 0) ; server and client
  (Components|DestroyComponent (Variables|Default|GetGems)) ; keep actor so functionality will still work
)

(event Custom|Server_AddGems
  (params (Target :type Actor%20Object%20Reference))
  ;[1 1 1] Add & update Gems UI
  (bind _asbp_pc_main_controller (Utilities|Casting|CastToBP_PC_MainController (Game|GetInstigatorController Target))))

(event Custom|Server_GiveKeyToPlayer
  (params (Controller :type Controller%20Object%20Reference))
  ;[1 0.3958 0.3958] unifinished - giving a key
  (Utilities|Casting|CastToBP_PC_MainController Controller))

(fn ConstructionScript)