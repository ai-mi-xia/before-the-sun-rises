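; Gem pickup reserved for player 2 that raises the jump velocity of the character collecting it.
; On authority, overlap matches the controller's index in the game mode's player list against Player2Index, printing debug messages.
; A match boosts jump, calls the add-gems event, plays a sound and destroys the gem components, keeping the actor.
; Gem counting and key-giving events stop after their casts; stamina and widget logic is disconnected.
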(event OnComponentBeginOverlap(PickUpRadius)
  (params (OverlappedComponent :type Primitive%20Component%20Object%20Reference) (OtherActor :type Actor%20Object%20Reference) (OtherComp :type Primitive%20Component%20Object%20Reference) (OtherBodyIndex :type Integer) (bFromSweep :type Boolean) (SweepResult :type Hit%20Result%20Structure%20%28by%20ref%29))
  ;[1 1 1] Pickup Gem
  (Networking|SwitchHasAuthority
    (:Authority
      (bind _asbp_third_person_character (Utilities|Casting|CastToBP_ThirdPerson_Character OtherActor))
      (bind _asbp_pc_main_controller (Utilities|Casting|CastToBP_PC_MainController (Game|GetInstigatorController OtherActor)))
      (bind _asbp_gm_default (Utilities|Casting|CastToBP_GM_Default (Game|GetGameMode)))
      (Development|PrintString (Utilities|String|ToString(Integer) (Utilities|Array|FindItem (Variables|/Game/Blueprints/Framework/BP_GM_Default.BP_GM_Default_C|GetAllPlayerControllers _asbp_gm_default) _asbp_pc_main_controller)))
      (if (== (Utilities|Array|FindItem (Variables|/Game/Blueprints/Framework/BP_GM_Default.BP_GM_Default_C|GetAllPlayerControllers _asbp_gm_default) _asbp_pc_main_controller) (Variables|Default|GetPlayer2Index))
        (Development|PrintString "i am player 2") ; blue - overlapping character
        ;;[1 1 1] Change Jump Velocity of Character that picked it up
        (Variables|/Script/Engine.CharacterMovementComponent|SetJumpZVelocity (Variables|/Script/Engine.Character|GetCharacterMovement _asbp_third_person_character) (+ (Variables|/Script/Engine.CharacterMovementComponent|GetJumpZVelocity (Variables|/Script/Engine.Character|GetCharacterMovement _asbp_third_person_character)) 1e+02))
        (CallFunction|ServerAddGems OtherActor) ; issue here on spawn
        (Audio|PlaySound2D "/Engine/VREditor/Sounds/UI/Click_on_Button_Cue.Click_on_Button_Cue" 1.0 1.0 0.0 0 0) ; server and client
        (Components|DestroyComponent (Variables|Default|GetGems)) ; keep actor so functionality will still work
        (else
          (Development|PrintString "this is for player 2"))))))

(event Custom|Server_AddGems
  (params (Target :type Actor%20Object%20Reference))
  ;[1 1 1] Add & update Gems UI
  (bind _asbp_pc_main_controller (Utilities|Casting|CastToBP_PC_MainController (Game|GetInstigatorController Target))))

(event Custom|Server_GiveKeyToPlayer
  (params (Controller :type Controller%20Object%20Reference))
  ;[1 0.3958 0.3958] unifinished - giving a key
  (Utilities|Casting|CastToBP_PC_MainController Controller))

(fn ConstructionScript)