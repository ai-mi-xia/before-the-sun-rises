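; Bonus gem pickup actor that permanently raises a character's jump velocity when collected.
; On overlap it prints player IDs, boosts the character, calls a server add-gems event, plays a sound, and destroys its mesh and trigger while keeping the actor.
; The player-ID check and server gem-count logic are unfinished, so no gems are added.
; A separate event pushes a dropped gem along the camera's forward direction with a velocity-change impulse.
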(event OnComponentBeginOverlap(PickUpRadius)
  (params (OverlappedComponent :type Primitive%20Component%20Object%20Reference) (OtherActor :type Actor%20Object%20Reference) (OtherComp :type Primitive%20Component%20Object%20Reference) (OtherBodyIndex :type Integer) (bFromSweep :type Boolean) (SweepResult :type Hit%20Result%20Structure%20%28by%20ref%29))
  ;[1 1 1] Pickup Gem
  (bind _asbp_third_person_character (Utilities|Casting|CastToBP_ThirdPerson_Character OtherActor))
  (Development|PrintString (Utilities|String|ToString(Integer) (Variables|/Game/Blueprints/Character/BP_ThirdPerson_Character.BP_ThirdPerson_Character_C|GetSpawnGem_PlayerID _asbp_third_person_character)) true true "(R=1.000000,G=0.090821,B=0.160526,A=1.000000)" 5.0)
  (Development|PrintString (Utilities|String|ToString(Integer) (Variables|/Script/Engine.PlayerState|GetPlayerId (Variables|/Script/Engine.Pawn|GetPlayerState _asbp_third_person_character))))
  (if (== (Variables|/Game/Blueprints/Character/BP_ThirdPerson_Character.BP_ThirdPerson_Character_C|GetSpawnGem_PlayerID _asbp_third_person_character) (Variables|/Script/Engine.PlayerState|GetPlayerId (Variables|/Script/Engine.Pawn|GetPlayerState _asbp_third_person_character)))
    _
    (else
      _))
  ;;[1 1 1] Change Jump Velocity of Character that picked it up
  (bind _output_get (Variables|/Script/Engine.CharacterMovementComponent|SetJumpZVelocity (Variables|/Script/Engine.Character|GetCharacterMovement _asbp_third_person_character) (+ (Variables|/Script/Engine.CharacterMovementComponent|GetJumpZVelocity (Variables|/Script/Engine.Character|GetCharacterMovement _asbp_third_person_character)) 1e+02)))
  (CallFunction|ServerAddGems OtherActor) ; issue here on spawn
  (Audio|PlaySound2D "/Engine/VREditor/Sounds/UI/Click_on_Button_Cue.Click_on_Button_Cue" 1.0 1.0 0.0 0 0) ; server and client
  (Components|DestroyComponent (Variables|Default|GetGems)) ; keep actor so functionality will still work
)

(event Custom|Server_AddGems
  (params (Target :type Actor%20Object%20Reference))
  ;[1 1 1] Add & update Gems UI - does NOT add bonus gems on pickup
  (bind _asbp_pc_main_controller (Utilities|Casting|CastToBP_PC_MainController (Game|GetInstigatorController Target))))

(event Custom|Server_CheckActorName
  (params (Actor :type Actor%20Object%20Reference)))

(event Custom|PushPickupItemAway
  (bind _returnvalue (Game|GetPlayerCameraManager 0))
  (bind _returnvalue_2 (Camera|GetCameraRotation _returnvalue))
  (bind _returnvalue_3 (Math|Vector|GetForwardVector _returnvalue_2))
  ;[1 1 1] Push item away when dropped
  (Class|PrimitiveComponent|AddVelocityChangeImpulseatLocation (Variables|Default|GetGems) (* _returnvalue_3 2.5e+02) (+ (Transformation|GetActorLocation) (* _returnvalue_3 "15.000000,0,0")) "None"))

(fn ConstructionScript)