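; Main player controller for a networked flower-planting game, owning water and flower counts, HUD and prompt widgets, and sound effects.
; Left-click previews then plants flowers through server RPCs, spending water and updating the HUD via multicast.
; Flower milestones boost jump and movement and light bloom spots, where tree-petal events later remove log doors.
; Server, client and multicast events also handle character opacity and level sequences; the intro cutscene chain is disconnected.
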(event Custom|DecreaseCharaOpacity
  (params (Flower%20Water%20Cost :type Float%20%28double-precision%29))
  ;[0.9463 0.6073 1] Press F to Water & Spawn Flower
  ;;[1 1 1] Change character opacity when water is used
  (CallFunction|MultiDecreaseOpacity Flower%20Water%20Cost))

(event Custom|Multicast_CallHUD
  ;[0.9463 0.6073 1] Press F to Water & Spawn Flower
  ;;[1 1 1] Multicast Call HUD Event Dispatcher
  (Default|CallUpdateHUD))

(event Custom|IncreaseFlowerCount
  ;[0.9463 0.6073 1] Press F to Water & Spawn Flower
  ;;[1 1 1] Increase Flower Count
  (Variables|Default|SetFlowerCount (+ (Variables|Default|GetFlowerCount) 1)))

(event Custom|HideBloomSpot1
  ;[1 1 1] Hide Bloom spot - called in Player Character BP
  (bind _outactors (Actor|GetAllActorsOfClass "/Game/Blueprints/Interactables/BP_BloomTreeCollision.BP_BloomTreeCollision_C"))
  (for _array_element _outactors
    (bind _asbp_bloom_tree_collision (Utilities|Casting|CastToBP_BloomTreeCollision _array_element))
    (Rendering|SetVisibility (Variables|/Game/Blueprints/Interactables/BP_BloomTreeCollision.BP_BloomTreeCollision_C|GetBloomPointLight _asbp_bloom_tree_collision) false false)
    (Collision|SetCollisionEnabled (Variables|/Game/Blueprints/Interactables/BP_BloomTreeCollision.BP_BloomTreeCollision_C|GetBloomCollision _asbp_bloom_tree_collision) "NoCollision")
    (Components|Activation|Deactivate (Variables|/Game/Blueprints/Interactables/BP_BloomTreeCollision.BP_BloomTreeCollision_C|GetBloomParticle _asbp_bloom_tree_collision))))

(event Custom|Client_DrawHUD
  ;[0.6615 0.6615 0.6615] Setup
  ;;[1 1 1] Display HUD
  (bind _returnvalue (UserInterface|CreateWidget "/Game/Widgets/InGameHUD_WidgetBP.InGameHUD_WidgetBP_C"))
  (bind _output_get (Variables|Default|SetWPB_InGameHud _returnvalue))
  (UserInterface|Viewport|AddtoViewport _output_get 0))

(event Custom|MulticastIncreaseOpacity
  (params (Puddle%20Water :type Float%20%28double-precision%29))
  ;[1 1 1] Change character opacity when water is used
  (bind _asbp_third_person_character (Utilities|Casting|CastToBP_ThirdPerson_Character (Pawn|GetControlledPawn)))
  (Default|IncreaseCharacterOpacity _asbp_third_person_character Puddle%20Water))

(event Custom|Server_KeyPressed
  ;[0.9463 0.6073 1] Press F to Water & Spawn Flower
  ;;[1 1 1] If actor is vaild, this is the overlapping controller
  (Utilities|IsValid (Variables|Default|GetDrySpot_OverlappedActor)
    (:Is%20Valid
      (if (> (Variables|Default|GetWater) 0.0)
        (Variables|Default|SetNotEnoughWater false)
        (CallFunction|ServerFlowerVisibility)
        (bind _asbp_third_person_character (Utilities|Casting|CastToBP_ThirdPerson_Character (Pawn|GetControlledPawn)))
        (Default|ServerSpawnFlowerEmoji _asbp_third_person_character)
        (else
          (Variables|Default|SetNotEnoughWater true)
          (CallFunction|MulticastCallWaterAni)
          (CallFunction|ClientNoWaterSound))))))

(event Custom|SpawnTreePetals2
  ;[0.3557 1 0.4036] Tree Bloom
  ;;[1 1 1] Spawn Petals on Heart Emote 2
  (Utilities|IsValid (Variables|Default|GetBloomSpotOverlappedActor2)
    (:Is%20Valid
      (bind _outactors (Actor|GetAllActorsOfClass "/Game/Blueprints/Interactables/BP_BloomTree2.BP_BloomTree2_C"))
      (bind _asbp_bloom_tree_2 (Utilities|Casting|CastToBP_BloomTree2 (Utilities|Array|Get(acopy) _outactors)))
      (Rendering|SetVisibility (Variables|/Game/Blueprints/Interactables/BP_BloomTree2.BP_BloomTree2_C|GetPetals _asbp_bloom_tree_2) true false)
      (Default|ChangeSpawnRate _asbp_bloom_tree_2)
      (CallFunction|ServerStopHeartPulse)
      (Utilities|FlowControl|Delay 3.0)
      (CallFunction|HideBloomSpot2)
      (CallFunction|ServerRemoveLogDoors2)
      (Utilities|FlowControl|Delay 1.0)
      (Math|Integer|IncrementInt (Variables|Default|GetTreeCount)
        (:%20%20
          (Utilities|FlowControl|Delay 1.5)
          (CallFunction|MulticastCallHUD))))))

(event Custom|CheckFlowerCount
  ;[0.3557 1 0.4036] Tree Bloom
  ;;[1 1 1] Check to see if Flower Count is reached
  (if (== (Variables|Default|GetFlowerCount) 15)
    (Utilities|FlowControl|DoOnce false
      (:Completed
        (bind _asbp_third_person_character (Utilities|Casting|CastToBP_ThirdPerson_Character (Pawn|GetControlledPawn)))
        (bind _output_get (Variables|Default|SetAs%20BP%20Third%20Person%20Character _asbp_third_person_character))
        (Default|IncreaseJumpandMovement _output_get)
        (Audio|PlaySound2D "/Game/Assets/Audio/SFX_BloomSpotApepar_Cue.SFX_BloomSpotApepar_Cue" 1.0 1.0 0.0 0 0)
        (bind _outactors (Actor|GetAllActorsOfClass "/Game/Blueprints/Interactables/BP_BloomTreeCollision.BP_BloomTreeCollision_C"))
        (for _array_element _outactors
          (bind _asbp_bloom_tree_collision (Utilities|Casting|CastToBP_BloomTreeCollision _array_element))
          (Rendering|SetVisibility (Variables|/Game/Blueprints/Interactables/BP_BloomTreeCollision.BP_BloomTreeCollision_C|GetBloomPointLight _asbp_bloom_tree_collision) true false)
          (Components|Activation|Activate (Variables|/Game/Blueprints/Interactables/BP_BloomTreeCollision.BP_BloomTreeCollision_C|GetBloomParticle _asbp_bloom_tree_collision) false))))
    (elif (== (Variables|Default|GetFlowerCount) 30)
      (Utilities|FlowControl|DoOnce false
        (:Completed
          (Default|IncreaseJumpandMovement (Variables|Default|GetAs%20BP%20Third%20Person%20Character))))
      (elif (== (Variables|Default|GetFlowerCount) 45)
        (Utilities|FlowControl|DoOnce false
          (:Completed
            (Default|IncreaseJumpandMovement (Variables|Default|GetAs%20BP%20Third%20Person%20Character))))
        (elif (== (Variables|Default|GetFlowerCount) 60)
          (Utilities|FlowControl|DoOnce false
            (:Completed
              (Default|IncreaseJumpandMovement (Variables|Default|GetAs%20BP%20Third%20Person%20Character))
              (bind _outactor (Sequencer|Player|CreateLevelSequencePlayer "/Game/Sequences/S_BloomSpot2.S_BloomSpot2"))
              (Sequencer|Player|Play (Variables|/Script/LevelSequence.LevelSequenceActor|GetSequencePlayer _outactor) :!class /Script/MovieScene.MovieSceneSequencePlayer)
              (Audio|PlaySound2D "/Game/Assets/Audio/SFX_BloomSpotApepar_Cue.SFX_BloomSpotApepar_Cue" 1.0 1.0 0.0 0 0)
              (bind _outactors_2 (Actor|GetAllActorsOfClass "/Game/Blueprints/Interactables/BP_BloomTreeCollision2.BP_BloomTreeCollision2_C"))
              (bind _asbp_bloom_tree_collision_2 (Utilities|Casting|CastToBP_BloomTreeCollision2 (Utilities|Array|Get(acopy) _outactors_2)))
              (Rendering|SetVisibility (Variables|/Game/Blueprints/Interactables/BP_BloomTreeCollision2.BP_BloomTreeCollision2_C|GetBloomPointLight _asbp_bloom_tree_collision_2) true false)
              (Components|Activation|Activate (Variables|/Game/Blueprints/Interactables/BP_BloomTreeCollision2.BP_BloomTreeCollision2_C|GetBloomParticles _asbp_bloom_tree_collision_2) false)))
          (elif (== (Variables|Default|GetFlowerCount) 75)
            (Utilities|FlowControl|DoOnce false
              (:Completed
                (Default|IncreaseJumpandMovement (Variables|Default|GetAs%20BP%20Third%20Person%20Character))))))))))

(event Custom|IncreaseCharaOpacity
  (params (Puddle%20Water :type Float%20%28double-precision%29))
  ;[1 1 1] Change character opacity when water is used
  (CallFunction|MulticastIncreaseOpacity Puddle%20Water))

(event Custom|Multi_LogStuff
  (params (Actor :type Actor%20Object%20Reference))
  ;[1 1 1] Show logs that block tutorial area, called on BP_LeavingTutorial
  (bind _asbp_third_person_character (Utilities|Casting|CastToBP_ThirdPerson_Character (Pawn|GetControlledPawn (Game|GetInstigatorController Actor))))
  (Rendering|Debug|DrawDebugSphere (Transformation|GetActorLocation _asbp_third_person_character) 2e+03 12 "(R=1.000000,G=1.000000,B=1.000000,A=1.000000)" 0.0)
  (bind _outactors (Collision|SphereOverlapActors (Transformation|GetActorLocation _asbp_third_person_character) 2e+03 (Utilities|Array|MakeArray "ObjectTypeQuery1") "/Game/Blueprints/Interactables/BP_LogClose.BP_LogClose_C"))
  (for _array_element _outactors
    (Rendering|SetVisibility (Variables|/Script/Engine.Actor|GetRootComponent _array_element) true false)))

(event Custom|Multicast_CallWaterAni
  ;[0.9463 0.6073 1] Press F to Water & Spawn Flower
  ;;[1 1 1] Multicast Call when no water
  (Default|CallUpdateWaterAni))

(event Custom|Multi_DecreaseOpacity
  (params (Flower%20Water%20Cost :type Float%20%28double-precision%29))
  ;[0.9463 0.6073 1] Press F to Water & Spawn Flower
  ;;[1 1 1] Change character opacity when water is used
  (bind _asbp_third_person_character (Utilities|Casting|CastToBP_ThirdPerson_Character (Pawn|GetControlledPawn)))
  (Default|DecreaseCharacterOpacity _asbp_third_person_character Flower%20Water%20Cost))

(event Custom|Client_PressHeartUI
  (bind _emote_wbp (Variables|Default|GetEmote_WBP))
  ;[0.7066 1 0.3534] BloomSpot UI
  ;;[1 1 1] Bloom spot- add
  (Widget|SetVisibility (Variables|/Game/Widgets/Emote_WBP.Emote_WBP_C|GetHeartBorder _emote_wbp) "Visible")
  (UserInterface|Animation|PlayAnimation _emote_wbp (Variables|/Game/Widgets/Emote_WBP.Emote_WBP_C|GetHeartPulseBig _emote_wbp) 0.0 20 "Forward" 1.0 false))

(event Custom|Server_PressHeartUI
  ;[0.7066 1 0.3534] BloomSpot UI
  ;;[1 1 1] Bloom spot- add
  (CallFunction|ClientPressHeartUI))

(event Custom|Client_StopHeartPulse
  (bind _emote_wbp (Variables|Default|GetEmote_WBP))
  ;[0.7066 1 0.3534] BloomSpot UI
  ;;[1 1 1] Bloom Spot - Remove
  (Class|UserWidget|StopAnimation _emote_wbp (Variables|/Game/Widgets/Emote_WBP.Emote_WBP_C|GetHeartPulseBig _emote_wbp))
  (Widget|SetVisibility (Variables|/Game/Widgets/Emote_WBP.Emote_WBP_C|GetHeartBorder _emote_wbp) "Hidden"))

(event Custom|Server_StopHeartPulse
  ;[0.7066 1 0.3534] BloomSpot UI
  ;;[1 1 1] Bloom Spot - Remove
  (CallFunction|ClientStopHeartPulse))

(event Custom|Server_FlowerVisibility
  ;[0.9463 0.6073 1] Press F to Water & Spawn Flower
  ;;[1 1 1] Set Spawn Location Visibility when F is pressed
  (bind _asbp_third_person_character (Utilities|Casting|CastToBP_ThirdPerson_Character (Variables|Default|GetDrySpot_OverlappedActor)))
  (Rendering|SetVisibility (Variables|/Game/Blueprints/Character/BP_ThirdPerson_Character.BP_ThirdPerson_Character_C|GetFlowerSpawn _asbp_third_person_character) true false))

(event Custom|Client_AddFlowerUI
  ;[0.9463 0.6073 1] Press F to Water & Spawn Flower
  ;;[1 1 1] Plant Flower UI - add
  (Utilities|IsValid (Variables|Default|GetFlower_WBP)
    (:Is%20Valid
      (Widget|SetVisibility (Variables|/Game/Widgets/Interact_UI/PlantFlowers_WBP.PlantFlowers_WBP_C|GetUI_ClickFlower (Variables|Default|GetFlower_WBP)) "Visible")
      (UserInterface|Animation|PlayAnimation (Variables|Default|GetFlower_WBP) (Variables|/Game/Widgets/Interact_UI/PlantFlowers_WBP.PlantFlowers_WBP_C|GetPulsing (Variables|Default|GetFlower_WBP)) 0.0 1 "Forward" 1.0 false))
    (:Is%20Not%20Valid
      (bind _returnvalue (UserInterface|CreateWidget "/Game/Widgets/Interact_UI/PlantFlowers_WBP.PlantFlowers_WBP_C"))
      (Variables|Default|SetFlower_WBP _returnvalue)
      (UserInterface|Viewport|AddtoViewport (Variables|Default|GetFlower_WBP) 0))))

(event Custom|Server_LogStuff
  (params (Actor :type Actor%20Object%20Reference))
  ;[1 1 1] Show logs that block tutorial area, called on BP_LeavingTutorial
  (CallFunction|MultiLogStuff Actor))

(event Custom|Server_AddFlowerUI
  ;[0.9463 0.6073 1] Press F to Water & Spawn Flower
  ;;[1 1 1] Plant Flower UI - add
  (CallFunction|ClientAddFlowerUI))

(event Custom|Client_RemoveFlowerUI
  (bind _flower_wbp (Variables|Default|GetFlower_WBP))
  ;[0.9463 0.6073 1] Press F to Water & Spawn Flower
  ;;[1 1 1] Plant Flower UI - Remove
  (Widget|SetVisibility (Variables|/Game/Widgets/Interact_UI/PlantFlowers_WBP.PlantFlowers_WBP_C|GetUI_ClickFlower _flower_wbp) "Hidden")
  (Class|UserWidget|StopAnimation _flower_wbp (Variables|/Game/Widgets/Interact_UI/PlantFlowers_WBP.PlantFlowers_WBP_C|GetPulsing _flower_wbp)))

(event Custom|Server_RemoveFlowerUI
  ;[0.9463 0.6073 1] Press F to Water & Spawn Flower
  ;;[1 1 1] Plant Flower UI - Remove
  (CallFunction|ClientRemoveFlowerUI))

(event Custom|Client_ChangeWaterLight
  (params (Owner :type Actor%20Object%20Reference))
  ;[0.3033 0.6336 1] Change BP WaterLight on Overlap, called in the puddles
  (Rendering|Components|Light|SetIntensity (Actor|GetComponentbyClass Owner "/Script/Engine.PointLightComponent") 0.0))

(event Custom|Client_JumpUI
  ;[1 1 1] Jump controls, called by Jump trigger box BP
  (Utilities|IsValid (Variables|Default|GetJumpWBP)
    (:Is%20Not%20Valid
      (bind _returnvalue (UserInterface|CreateWidget "/Game/Widgets/Interact_UI/Jump_WBP.Jump_WBP_C"))
      (bind _output_get (Variables|Default|SetJumpWBP _returnvalue))
      (UserInterface|Viewport|AddtoViewport _output_get 0)
      (UserInterface|Animation|PlayAnimation (Variables|Default|GetJumpWBP) (Variables|/Game/Widgets/Interact_UI/Jump_WBP.Jump_WBP_C|GetSpaceJump (Variables|Default|GetJumpWBP)) 0.0 20 "Forward" 1.0 false)
      (Utilities|FlowControl|Delay 3.0)
      (Widget|RemovefromParent (Variables|Default|GetJumpWBP)))))

(event Custom|Client_RemoveJumpUI
  ;[1 1 1] Jump controls, called by Jump trigger box BP
  ;;[1 1 1] Not working - widget not getting removed
  (Widget|RemovefromParent (Variables|Default|GetJumpWBP)))

(event Custom|Server_RemoveLogDoors2
  ;[1 1 1] Main Log Door - replicated
  (CallFunction|MultiRemoveLogDoors2))

(event Custom|EmoteWidget_Server
  ;[1 1 1] Add emote to viewport
  (CallFunction|EmoteWidgetClient))

(event Custom|EmoteWidget_Client
  ;[1 1 1] Add emote to viewport
  (bind _returnvalue (UserInterface|CreateWidget "/Game/Widgets/Emote_WBP.Emote_WBP_C"))
  (bind _output_get (Variables|Default|SetEmote_WBP _returnvalue))
  (UserInterface|Viewport|AddtoViewport _output_get 0))

(event Custom|Server_Show%20Chara
  ;[1 1 1] Hide and Show Character
  (bind _asbp_third_person_character (Utilities|Casting|CastToBP_ThirdPerson_Character (Pawn|GetControlledPawn)))
  (Rendering|SetVisibility (Variables|/Script/Engine.Character|GetMesh _asbp_third_person_character) true false))

(event Custom|Server_IntroCutscene
  ;[1 1 1] Intro Cutscene Widget
  (CallFunction|ClientIntroCutscene))

(event Custom|Client_NoWaterSound
  ;[1 0.2686 0.7041] SFX
  ;;[1 1 1] No water SFX
  (Audio|PlaySound2D "/Game/Assets/Audio/Audio/NoWaterError_SFX_Cue.NoWaterError_SFX_Cue" 1.0 1.0 0.0 0 0))

(event Custom|Server_PlantFlowerSound
  ;[1 0.2686 0.7041] SFX
  ;;[1 1 1] Plant Flower SFX
  (CallFunction|MulticastPlantFlowerSound))

(event Custom|Multicast_PlantFlowerSound
  ;[1 0.2686 0.7041] SFX
  ;;[1 1 1] Plant Flower SFX
  (Audio|PlaySoundatLocation "/Game/Assets/Audio/Audio/PlantFlower_SFX_Cue.PlantFlower_SFX_Cue" (Transformation|GetActorLocation (Pawn|GetControlledPawn)) "0, 0, 0" 1.0 1.0 0.0 "/Game/Blueprints/Sound/Attenuation_Environment.Attenuation_Environment" 0 0 0))

(event Custom|SpawnTreePetals
  ;[0.3557 1 0.4036] Tree Bloom
  ;;[1 1 1] Spawn Petals on Heart Emote
  (Utilities|IsValid (Variables|Default|GetBloomSpot_OverlappedActor)
    (:Is%20Valid
      (bind _outactors (Actor|GetAllActorsOfClass "/Game/Blueprints/Interactables/BP_BloomTree.BP_BloomTree_C"))
      (for _array_element _outactors
        (bind _asbp_bloom_tree (Utilities|Casting|CastToBP_BloomTree _array_element))
        (Rendering|SetVisibility (Variables|/Game/Blueprints/Interactables/BP_BloomTree.BP_BloomTree_C|GetPetals _asbp_bloom_tree) true false)
        (Default|ChangeSpawnRate _asbp_bloom_tree)
        (CallFunction|ServerStopHeartPulse)
        (Utilities|FlowControl|Delay 5.0)
        (CallFunction|HideBloomSpot1)
        (CallFunction|RemoveLogDoors)
        (Math|Integer|IncrementInt (Variables|Default|GetTreeCount)
          (:%20%20
            (Utilities|FlowControl|Delay 1.5)
            ;[0.7066 1 0.3534] BloomSpot UI
            ;;[1 1 1] Bloom spot- add
            (CallFunction|MulticastCallHUD)))))))

(event Custom|HideBloomSpot2
  ;[1 1 1] Hide Bloom spot - called in Player Character BP
  (Utilities|FlowControl|DoOnce false
    (:Completed
      (bind _outactors (Actor|GetAllActorsOfClass "/Game/Blueprints/Interactables/BP_BloomTreeCollision2.BP_BloomTreeCollision2_C"))
      (bind _asbp_bloom_tree_collision_2 (Utilities|Casting|CastToBP_BloomTreeCollision2 (Utilities|Array|Get(acopy) _outactors)))
      (Rendering|SetVisibility (Variables|/Game/Blueprints/Interactables/BP_BloomTreeCollision2.BP_BloomTreeCollision2_C|GetBloomPointLight _asbp_bloom_tree_collision_2) false false)
      (Components|Activation|Deactivate (Variables|/Game/Blueprints/Interactables/BP_BloomTreeCollision2.BP_BloomTreeCollision2_C|GetBloomParticles _asbp_bloom_tree_collision_2))
      (Collision|SetCollisionEnabled (Variables|/Game/Blueprints/Interactables/BP_BloomTreeCollision2.BP_BloomTreeCollision2_C|GetBloomCollision _asbp_bloom_tree_collision_2) "NoCollision"))))

(event Custom|RemoveLogDoors
  ;[1 1 1] Remove tutorial log doors
  (CallFunction|MultiRemoveLogDoors))

(event Custom|Multi_RemoveLogDoors
  ;[1 1 1] Remove tutorial log doors
  (Audio|PlaySound2D "/Game/Assets/Audio/SFX_SuccessLog_Cue.SFX_SuccessLog_Cue" 1.0 1.0 0.0 0 0)
  (bind _asbp_third_person_character (Utilities|Casting|CastToBP_ThirdPerson_Character (Pawn|GetControlledPawn)))
  (bind _outactors (Collision|SphereOverlapActors (Transformation|GetActorLocation _asbp_third_person_character) 5e+03 (Utilities|Array|MakeArray "ObjectTypeQuery1") "/Game/Blueprints/Interactables/BP_LogDoor.BP_LogDoor_C"))
  (for _array_element _outactors
    (Actor|DestroyActor _array_element)))

(event Custom|Multi_RemoveLogDoors2
  ;[1 1 1] Main Log Door - replicated
  (Audio|PlaySound2D "/Game/Assets/Audio/SFX_SuccessLog_Cue.SFX_SuccessLog_Cue" 1.0 1.0 0.0 0 0)
  (bind _outactors (Actor|GetAllActorsOfClass "/Game/Blueprints/Interactables/BP_LogDoor2.BP_LogDoor2_C"))
  (for _array_element _outactors
    (Actor|DestroyActor _array_element)))

(event Custom|ChangeFlowerCount
  ;[0.9463 0.6073 1] Press F to Water & Spawn Flower
  ;;[1 0.4301 0.6021] Change Flower Count -??? not in use
  (bind _outactors (Actor|GetAllActorsOfClass "/Game/Blueprints/Interactables/BP_DrySpot_Parent.BP_DrySpot_Parent_C"))
  (bind _asbp_dry_spot_parent (Utilities|Casting|CastToBP_DrySpot_Parent (Utilities|Array|Get(acopy) _outactors)))
  (bind _output_get (Variables|Default|SetMaxFlowersReached? (>= (Variables|Default|GetNumFlowersSpawned) (Variables|/Game/Blueprints/Interactables/BP_DrySpot_Parent.BP_DrySpot_Parent_C|GetMaxFlowerNum _asbp_dry_spot_parent))))
  (if (not _output_get)
    (Variables|Default|SetNumFlowersSpawned (+ (Variables|Default|GetNumFlowersSpawned) 1))))

(event Custom|Client_IntroCutscene
  ;[1 1 1] Intro Cutscene Widget
  (bind _returnvalue (UserInterface|CreateWidget "/Game/Widgets/WBP_IntroCutscene.WBP_IntroCutscene_C"))
  (UserInterface|Viewport|AddtoViewport _returnvalue 0)
  (Utilities|FlowControl|Delay 18.0)
  (UserInterface|Animation|PlayAnimation _returnvalue (Variables|/Game/Widgets/WBP_IntroCutscene.WBP_IntroCutscene_C|GetFade _returnvalue) 0.0 1 "Forward" 1.0 false))

(event Custom|Client_WaterDropSFX
  ;[1 0.2686 0.7041] SFX
  ;;[1 1 1] Water SFX, called on puddle BP
  (Audio|PlaySound2D "/Game/Assets/Audio/Audio/CollecteWater_SFX_Cue.CollecteWater_SFX_Cue" 1.0 1.0 0.0 0 0))

(event Custom|Add%20Movement%20Widget%20on%20Server
  ;[1 1 1] UI - Movement controls on event begin play
  (CallFunction|AddWidgetonClient))

(event Custom|Add%20Widget%20on%20Client
  ;[1 1 1] UI - Movement controls on event begin play
  (bind _returnvalue (UserInterface|CreateWidget "/Game/Widgets/Interact_UI/MovementControls_WBP.MovementControls_WBP_C"))
  (UserInterface|Viewport|AddtoViewport _returnvalue 0)
  (UserInterface|Animation|PlayAnimation _returnvalue (Variables|/Game/Widgets/Interact_UI/MovementControls_WBP.MovementControls_WBP_C|GetFadeOut _returnvalue) 0.0 1 "Forward" 1.0 false)
  (Utilities|FlowControl|Delay 5.0)
  (Widget|RemovefromParent _returnvalue))

(event Custom|Server_PlayWaterCollectSound
  ;[1 0.2686 0.7041] SFX
  ;;[1 1 1] Water SFX, called on puddle BP
  (CallFunction|MultiWaterCollectedSFX))

(event Custom|Multi_WaterCollectedSFX
  ;[1 0.2686 0.7041] SFX
  ;;[1 1 1] Water SFX, called on puddle BP
  (Audio|PlaySoundatLocation "/Game/Assets/Audio/Audio/CollecteWater_SFX_Cue.CollecteWater_SFX_Cue" (Transformation|GetActorLocation (Pawn|GetControlledPawn)) "0, 0, 0" 1.0 1.0 0.0 "/Game/Blueprints/Sound/Attenuation_Environment.Attenuation_Environment" 0 0 0))

(event Custom|Server_HideChara
  ;[1 1 1] Hide and Show Character
  (bind _asbp_third_person_character (Utilities|Casting|CastToBP_ThirdPerson_Character (Pawn|GetControlledPawn)))
  (Rendering|SetVisibility (Variables|/Script/Engine.Character|GetMesh _asbp_third_person_character) false false))

(event Custom|Server_Level1EndSequence
  ;[1 1 1] End Sequence, called from third person BP
  (CallFunction|MultiLevel1EndSequence))

(event Custom|Multi_Level1EndSequence
  ;[1 1 1] End Sequence, called from third person BP
  (bind _outactor (Sequencer|Player|CreateLevelSequencePlayer "/Game/Sequences/S_Level1BloomTree.S_Level1BloomTree"))
  (Sequencer|Player|Play (Variables|/Script/LevelSequence.LevelSequenceActor|GetSequencePlayer _outactor) :!class /Script/MovieScene.MovieSceneSequencePlayer))

(event Custom|Server_SpawnFlower
  ;[0.9463 0.6073 1] Press F to Water & Spawn Flower
  ;;[1 1 1] Spawn Flower when F is released AND is not overlapping any other flowers
  (bind _asbp_third_person_character (Utilities|Casting|CastToBP_ThirdPerson_Character (Variables|Default|GetDrySpot_OverlappedActor)))
  (if (or (Variables|/Game/Blueprints/Character/BP_ThirdPerson_Character.BP_ThirdPerson_Character_C|GetDoNotSpawnFlower _asbp_third_person_character) (Variables|Default|GetNotEnoughWater))
    (Rendering|SetVisibility (Variables|/Game/Blueprints/Character/BP_ThirdPerson_Character.BP_ThirdPerson_Character_C|GetFlowerSpawn _asbp_third_person_character) false false)
    (else
      (Game|SpawnActorfromClass "/Game/Blueprints/Interactables/BP_Flowers.BP_Flowers_C" (Transformation|GetWorldTransform (Variables|/Game/Blueprints/Character/BP_ThirdPerson_Character.BP_ThirdPerson_Character_C|GetFlowerSpawn _asbp_third_person_character)) "DontSpawnIfColliding" 0 0)
      (Rendering|SetVisibility (Variables|/Game/Blueprints/Character/BP_ThirdPerson_Character.BP_ThirdPerson_Character_C|GetFlowerSpawn _asbp_third_person_character) false false)
      (CallFunction|DecreaseWater)
      (CallFunction|IncreaseFlowerCount)
      (CallFunction|MulticastCallHUD)
      (CallFunction|ServerPlantFlowerSound))))

(event Custom|DecreaseWater
  ;[0.9463 0.6073 1] Press F to Water & Spawn Flower
  ;;[1 1 1] Decrease Water
  (Variables|Default|SetWater (- (Variables|Default|GetWater) 1.0)))

(event EventBeginPlay
  ;[0.6615 0.6615 0.6615] Setup
  ;;[1 1 1] Hide Mouse
  (if (Pawn|IsLocalPlayerController)
    (Input|SetInputModeGameOnly self)
    (Variables|Default|SetbShowMouseCursor false)
    (Viewport|RemoveAllWidgets)
    (CallFunction|ClientDrawHUD)
    (CallFunction|AddMovementWidgetonServer)
    (CallFunction|EmoteWidgetServer)
    (Input|EnableInput (Pawn|GetControlledPawn) 0)))

(event Input|ActionEvents|InputActionMouseClickLeft
  (params (Key :type Key%20Structure :default "None"))
  ;[0.9463 0.6073 1] Press F to Water & Spawn Flower
  ;;[1 1 1] Input, Call server RPC
  (:Pressed
    (CallFunction|ServerKeyPressed))
  (:Released
    (CallFunction|ServerSpawnFlower)
    (Utilities|FlowControl|Delay 0.2)
    (CallFunction|CheckFlowerCount)))

(fn ConstructionScript)

(fn OnRepFIsPressed?)

(fn OnRepUpdateHUD)

(fn OnRepWater)