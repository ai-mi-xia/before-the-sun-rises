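; Menu game mode that runs the lobby and starts the match once enough players have joined.
; When a new player enters on the Lobby Map, it stores their BP_PC_MenuController and has it create the lobby menu.
; At two or more connected players, it updates the newest controller's waiting text and has BP_GameInstance travel to the hard-coded first level.
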(event EventBeginPlay)

(event EventTick
  (params (DeltaSeconds :type Float%20%28single-precision%29)))

(event EventHandleStartingNewPlayer
  (params (NewPlayer :type Player%20Controller%20Object%20Reference))
  ;[1 1 1] Execute when new player enters
  (bind _returnvalue (Game|GetCurrentLevelName true))
  (switch string _returnvalue
    (:Lobby_Map
      (bind _asbp_pc_menu_controller (Utilities|Casting|CastToBP_PC_MenuController NewPlayer))
      (Utilities|Array|Add (Variables|Default|GetAllConnectedPlayers) _asbp_pc_menu_controller)
      (Default|CreateLobbyMenu _asbp_pc_menu_controller)
      (if (>= (Utilities|Array|Length (Variables|Default|GetAllConnectedPlayers)) 2)
        (Default|ServerUIChangeWaitingText _asbp_pc_menu_controller)
        (bind _asbp_game_instance (Utilities|Casting|CastToBP_GameInstance (Game|GetGameInstance)))
        (Default|TraveltoMap _asbp_game_instance 2 "Level1_WB_WP_2")))))

(fn ConstructionScript)